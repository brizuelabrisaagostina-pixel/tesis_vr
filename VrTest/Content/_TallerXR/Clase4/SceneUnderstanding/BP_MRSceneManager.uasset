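; Mixed reality scene manager that loads the device's room scan through MRUK on BeginPlay, after a short delay.
; If loading fails it launches a space setup capture, and a successful capture-complete callback triggers another load.
; A separate event queries saved Oculus spatial anchors and spawns BP_SpatialAnchorMarker at each, but its only call here is disconnected.
; On-screen Spanish messages report the results.
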(event Custom|IniciarEscaneoHabitacion
  (bind _returnvalue (Class|MRUKSubsystem|LaunchSceneCapture (Subsystems|GetMRUKSubsystem)))
  (if _returnvalue
    (Development|PrintString "ESCANEO ESPACIAL INICIADO" true true "(R=0.000000,G=1.000000,B=0.044453,A=1.000000)" 5.0)
    (else
      (Development|PrintString "NO SE PUDO INICIAR EL ESCANEO" true true "(R=1.000000,G=0.011515,B=0.000000,A=1.000000)" 5.0))))

(event Custom|CargarEscenaMR
  (|LoadScenefromDeviceAsync "V1"
    (:Success
      (Development|PrintString "ESCENA MR CARGADA" true true "(R=0.000000,G=1.000000,B=0.044453,A=1.000000)" 5.0))
    (:Failure
      (Development|PrintString "ERROR AL CARGAR ESCENA MR" true true "(R=1.000000,G=0.011515,B=0.000000,A=1.000000)" 5.0)
      (CallFunction|IniciarEscaneoHabitacion))))

(event Custom|OnCaptureComplete_Event
  (params (Success :type Boolean))
  (if Success
    (Utilities|FlowControl|Delay 0.5)
    (CallFunction|CargarEscenaMR)
    (else
      (Development|PrintString "EL ESCANEO ESPACIAL FUE CANCELADO O FALLÓ" true true "(R=1.000000,G=0.011515,B=0.000000,A=1.000000)" 5.0))))

(event Custom|CargarAnclasGuardadas
  (bind _queryresults (|OculusXRAsyncQueryAnchorsAdvanced (Utilities|Struct|MakeOculusXRSpaceQueryInfo 100 0.0 "Local" "None" 0 "Locatable"))
    (:Success
      (for _array_element _queryresults
        (Class|OculusXRAnchorBPFunctionLibrary|SpawnActorwithAnchorQueryResults _array_element "/Game/_TallerXR/Clase4/SceneUnderstanding/BP_SpatialAnchorMarker.BP_SpatialAnchorMarker_C" 0 0 "AlwaysSpawn"))
      (Development|PrintString "ANCLAS GUARDADAS RECUPERADAS" true true "(R=0.000000,G=1.000000,B=0.000798,A=1.000000)" 5.0))
    (:Failure
      (Development|PrintString "NO SE PUDIERON RECUPERAR LAS ANCLAS" true true "(R=1.000000,G=0.046073,B=0.000000,A=1.000000)" 5.0))))

(event EventBeginPlay
  (EventDispatchers|AssignOnCaptureComplete (Subsystems|GetMRUKSubsystem) (delegate Custom|OnCaptureComplete_Event))
  (Utilities|FlowControl|Sequence
    (:then_0
      (Utilities|FlowControl|Delay 1.0)
      (CallFunction|CargarEscenaMR))))

(fn ConstructionScript)