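; BP_Glass is a glass, filed with the XR workshop's pickeable objects, that can be filled with water and spills when tipped.
; It starts empty; FillGlass snaps the water mesh back to its origin and shows it with physics and collision off.
; While filled, Tick compares the glass's up vector to world up with a dot product.
; Past roughly 60 degrees of tilt, SpillWater detaches the water mesh and makes it a colliding physics body.
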(event EventBeginPlay
  (|CallParentFunction)
  (CallFunction|SetGlassState false))

(event EventTick
  (params (DeltaSeconds :type Float%20%28single-precision%29))
  (|CallParentFunction DeltaSeconds)
  (if (Variables|Default|GetIsFilled)
    (if (< (Math|Vector|DotProduct (Math|Vector|GetUpVector (Variables|Default|GetObjectMesh)) "0.000000,0.000000,1.000000") 0.5)
      (CallFunction|SpillWater))))

(fn ConstructionScript
  (|CallParentFunction))

(fn SetGlassState
  (params (Fill? :type Boolean))
  (bind _watermesh (Variables|Default|GetWaterMesh))
  (bind _watermesh_2 (Variables|Default|GetWaterMesh))
  (Physics|SetSimulatePhysics _watermesh false)
  (Collision|SetCollisionEnabled _watermesh "NoCollision")
  (Transformation|AttachComponentToComponent _watermesh (Variables|Default|GetWaterOrigin) "None" "SnapToTarget" "SnapToTarget" "KeepWorld" true)
  (Transformation|SetRelativeLocationAndRotation _watermesh_2 "0, 0, 0" "0, 0, 0" false false)
  (bind _output_get (Variables|Default|SetIsFilled Fill?))
  (Rendering|SetVisibility _watermesh_2 _output_get false))

(fn SpillWater
  (bind _watermesh (Variables|Default|GetWaterMesh))
  (if (Variables|Default|GetIsFilled)
    (Variables|Default|SetIsFilled false)
    (Transformation|DetachFromComponent _watermesh "KeepWorld" "KeepWorld" "KeepWorld" true)
    (Collision|SetCollisionEnabled _watermesh "QueryAndPhysics")
    (Physics|SetSimulatePhysics _watermesh true)))

(fn FillGlass
  (if (not (Variables|Default|GetIsFilled))
    (CallFunction|SetGlassState true)))