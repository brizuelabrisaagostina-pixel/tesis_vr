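; BP_Faucet is an interactable VR faucet that fills a glass the player is holding.
; On Interactuar it casts the interactor to BP_VRPawn_Clase3, then checks the left held component and, failing that, the right.
; TryFillHeldGlass casts the component's owner to BP_Glass, calls FillGlass and returns whether it succeeded.
; If neither hand holds a glass, it prints a debug message.
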(event EventBeginPlay
  (|CallParentFunction) ; This node is disabled and will not be called.\nDrag off pins to build functionality.
)

(event Collision|EventActorBeginOverlap
  (params (OtherActor :type Actor%20Object%20Reference))
  (|CallParentFunction OtherActor) ; This node is disabled and will not be called.\nDrag off pins to build functionality.
)

(event EventTick
  (params (DeltaSeconds :type Float%20%28single-precision%29))
  (|CallParentFunction DeltaSeconds) ; This node is disabled and will not be called.\nDrag off pins to build functionality.
)

(event EventInteractuar
  (params (Interactor :type Actor%20Object%20Reference))
  (bind _asbp_vrpawn_clase_3 (Utilities|Casting|CastToBP_VRPawn_Clase3 Interactor))
  (bind _foundglass (CallFunction|TryFillHeldGlass (Variables|/Game/_TallerXR/Clase3/2_Interactions/BP_VRPawn_Clase3.BP_VRPawn_Clase3_C|GetHeldComponentLeft _asbp_vrpawn_clase_3)))
  (if (not _foundglass)
    (bind _foundglass_2 (CallFunction|TryFillHeldGlass (Variables|/Game/_TallerXR/Clase3/2_Interactions/BP_VRPawn_Clase3.BP_VRPawn_Clase3_C|GetHeldComponentRight _asbp_vrpawn_clase_3)))
    (if (not _foundglass_2)
      (Development|PrintString "No hay vaso agarrado"))))

(fn ConstructionScript
  (|CallParentFunction))

(fn TryFillHeldGlass
  (params (HeldComponent :type Actor%20Component%20Object%20Reference))
  (Utilities|IsValid HeldComponent
    (:Is%20Valid
      (bind _asbp_glass (Utilities|Casting|CastToBP_Glass (Components|GetOwner HeldComponent))
        (:then
          (Default|FillGlass _asbp_glass)
          (return true))
        (:CastFailed
          _)))
    (:Is%20Not%20Valid
      _))
  (return false))