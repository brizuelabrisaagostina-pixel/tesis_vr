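; BP_LightSwitch is an interactable light switch that turns a target light on or off.
; Its Interactuar event validates the LuzObjetivo reference, gets that actor's PointLightComponent and toggles its visibility without propagating to child components.
; The switch holds no state of its own; BeginPlay, overlap and Tick are disabled stubs, and the construction script only calls its parent.
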(event EventBeginPlay
  (|CallParentFunction) ; This node is disabled and will not be called.\nDrag off pins to build functionality.
)

(event Collision|EventActorBeginOverlap
  (params (OtherActor :type Actor%20Object%20Reference))
  (|CallParentFunction OtherActor) ; This node is disabled and will not be called.\nDrag off pins to build functionality.
)

(event EventTick
  (params (DeltaSeconds :type Float%20%28single-precision%29))
  (|CallParentFunction DeltaSeconds) ; This node is disabled and will not be called.\nDrag off pins to build functionality.
)

(event EventInteractuar
  (params (Interactor :type Actor%20Object%20Reference))
  (bind _luzobjetivo (Variables|Default|GetLuzObjetivo))
  (Utilities|IsValid _luzobjetivo
    (:Is%20Valid
      (Rendering|ToggleVisibility (Actor|GetComponentbyClass _luzobjetivo "/Script/Engine.PointLightComponent") false))))

(fn ConstructionScript
  (|CallParentFunction))