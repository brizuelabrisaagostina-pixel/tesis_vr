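; BP_NotPickeable_Base is a base actor for non-pickable interactable objects, providing highlight and prompt feedback for interaction.
; On BeginPlay it hides the InteractionIndicator widget component and sets its prompt text.
; Events and MostrarOcultarFeedback toggle an overlay highlight material and the indicator; the highlight events also toggle custom depth.
; While the indicator is visible, Tick rotates it to face the player camera.
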(event EventBeginPlay
  (Rendering|SetVisibility (Variables|Default|GetInteractionIndicator) false false)
  (bind _aswbp_interaction_prompt (Utilities|Casting|CastToWBP_InteractionPrompt (UserInterface|GetUserWidgetObject (Variables|Default|GetInteractionIndicator))))
  (Default|SetPromptText _aswbp_interaction_prompt (Variables|Default|GetPromptText)))

(event Collision|EventActorBeginOverlap
  (params (OtherActor :type Actor%20Object%20Reference)))

(event EventTick
  (params (DeltaSeconds :type Float%20%28single-precision%29))
  (if (Rendering|IsVisible (Variables|Default|GetInteractionIndicator))
    (CallFunction|UpdatePromptRotation)))

(event EventMostrarHighlight
  (bind _objectmesh (Variables|Default|GetObjectMesh))
  (Rendering|SetRenderCustomDepth _objectmesh true)
  (Rendering|Material|SetOverlayMaterial _objectmesh "/Game/_TallerXR/Clase3/Materials/M_InteractionHighlight.M_InteractionHighlight" :!class /Script/Engine.MeshComponent))

(event EventOcultarIndicador
  (Rendering|SetVisibility (Variables|Default|GetInteractionIndicator) false false))

(event EventMostrarIndicador
  (Rendering|SetVisibility (Variables|Default|GetInteractionIndicator) true false))

(event EventOcultarHighlight
  (bind _objectmesh (Variables|Default|GetObjectMesh))
  (Rendering|SetRenderCustomDepth _objectmesh false)
  (Rendering|Material|SetOverlayMaterial _objectmesh 0 :!class /Script/Engine.MeshComponent))

(fn ConstructionScript)

(fn UpdatePromptRotation
  (Transformation|SetWorldRotation (Variables|Default|GetInteractionIndicator) (Math|Rotator|FindLookatRotation (Transformation|GetWorldLocation (Variables|Default|GetInteractionIndicator)) (Camera|GetCameraLocation (Game|GetPlayerCameraManager 0))) false false))

(fn MostrarOcultarFeedback
  (params (Mostrar :type Boolean))
  (bind _objectmesh (Variables|Default|GetObjectMesh))
  (if Mostrar
    (Rendering|Material|SetOverlayMaterial _objectmesh "/Game/_TallerXR/Clase3/Materials/M_InteractionHighlight.M_InteractionHighlight" :!class /Script/Engine.MeshComponent)
    (else
      (Rendering|Material|SetOverlayMaterial _objectmesh 0 :!class /Script/Engine.MeshComponent)))
  (Rendering|SetVisibility (Variables|Default|GetInteractionIndicator) Mostrar false))