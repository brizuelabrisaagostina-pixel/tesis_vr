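; BP_DoorHandle is an interactable door handle that toggles the door it belongs to.
; Its Interactuar event casts the parent actor to BP_Door and calls AlternarPuerta, so it expects to be a child actor of that door.
; If the cast fails nothing happens, and the handle has no other active logic.
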(event EventBeginPlay
  (|CallParentFunction) ; This node is disabled and will not be called.\nDrag off pins to build functionality.
)

(event Collision|EventActorBeginOverlap
  (params (OtherActor :type Actor%20Object%20Reference))
  (|CallParentFunction OtherActor) ; This node is disabled and will not be called.\nDrag off pins to build functionality.
)

(event EventTick
  (params (DeltaSeconds :type Float%20%28single-precision%29))
  (|CallParentFunction DeltaSeconds) ; This node is disabled and will not be called.\nDrag off pins to build functionality.
)

(event EventInteractuar
  (params (Interactor :type Actor%20Object%20Reference))
  (bind _asbp_door (Utilities|Casting|CastToBP_Door (Actor|GetParentActor)))
  (Default|AlternarPuerta _asbp_door))

(fn ConstructionScript
  (|CallParentFunction))